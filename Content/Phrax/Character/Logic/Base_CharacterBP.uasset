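; Base character Blueprint that derives per-frame movement state: acceleration, horizontal speed, movement input amount and aim yaw rate.
; Tick calls SetEssentialValues after the parent tick, also saving the last velocity and input rotations while each is active.
; Acceleration and yaw rate are meant as frame deltas against values from CacheValues, which this file never calls.
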(event EventBeginPlay
  ;[0.3851 1 0.3241] Event BeginPlay
  (|CallParentFunction))

(event EventTick
  (params (DeltaSeconds :type Float%20%28single-precision%29))
  (|CallParentFunction DeltaSeconds)
  ;[0.18 0.6 0.9] Do Every Frame
  (Utilities|FlowControl|Sequence
    (:then_0
      (EssentialInformation|SetEssentialValues))))

(fn ConstructionScript)

(fn SetEssentialValues
  (bind _returnvalue (Transformation|GetVelocity))
  (bind _charactermovement (Variables|Character|GetCharacterMovement))
  (Utilities|FlowControl|Sequence
    (:then_0
      ;[1 1 1] Set the amount of Acceleration.
      (Variables|Default|SetAcceleration (stale _returnvalue)))
    (:then_1
      ;[1 1 1] Determine if the character is moving by getting it's speed. The Speed equals the length of the horizontal (x y) velocity, so it does not take vertical movement into account. If the character is moving, update the last velocity rotation. This value is saved because it might be useful to know the last orientation of movement even after the character has stopped.
      (bind _output_get (Variables|Default|SetSpeed (Math|Vector|VectorLength (Math|Vector|MakeVector (.x _returnvalue) (.y _returnvalue) 0.0))))
      (bind _output_get_2 (Variables|Default|SetIsMoving (> _output_get 1.0)))
      (if _output_get_2
        (Variables|Default|SetLastVelocityRotation (Math|Conversions|RotationFromXVector (Transformation|GetVelocity)))))
    (:then_2
      ;[1 1 1] Determine if the character has movement input by getting its movement input amount. The Movement Input Amount is equal to the current acceleration divided by the max acceleration so that it has a range of 0-1, 1 being the maximum possible amount of input, and 0 beiung none. If the character has movement input, update the Last Movement Input Rotation.
      (bind _output_get_3 (Variables|Default|SetMovementInputAmount (/ (Math|Vector|VectorLength (Pawn|Components|CharacterMovement|GetCurrentAcceleration _charactermovement)) (Class|CharacterMovementComponent|GetMaxAcceleration _charactermovement))))
      (bind _output_get_4 (Variables|Default|SetHasMovementInput (> _output_get_3 0.0)))
      (if _output_get_4
        (Variables|Default|SetLastMovementInputRotation (Math|Conversions|RotationFromXVector (Pawn|Components|CharacterMovement|GetCurrentAcceleration (Variables|Character|GetCharacterMovement))))))
    (:then_3
      ;[1 1 1] Set the Aim Yaw rate by comparing the current and previous Aim Yaw value, divided by Delta Seconds. This represents the speed the camera is rotating left to right.
      (Variables|Default|SetAimYawRate (Math|Float|Absolute(Float) (/ (- (.yaw (Pawn|GetControlRotation :!class /Script/Engine.Pawn)) (Variables|CachedVariables|GetPreviousAimYaw)) (Utilities|Time|GetWorldDeltaSeconds)))))))

(fn CacheValues
  ;[1 1 1] Cache certain values to be used in calculations on the next frame
  (Utilities|FlowControl|Sequence
    (:then_0
      (Variables|CachedVariables|SetPreviousVelocity (Transformation|GetVelocity)))
    (:then_1
      (Variables|CachedVariables|SetPreviousAimYaw (.yaw (Pawn|GetControlRotation :!class /Script/Engine.Pawn))))))

(fn CalculateAcceleration
  ;[1 1 1] Calculate the Acceleration by comparing the current and previous velocity. The Current Acceleration returned by the movement component equals the input acceleration, and does not represent the actual physical acceleration of the character.
  (return (/ (- (Transformation|GetVelocity) (Variables|CachedVariables|GetPreviousVelocity)) (Utilities|Time|GetWorldDeltaSeconds))))